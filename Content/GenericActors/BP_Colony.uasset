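; BP_Colony is an actor that procedurally scatters placeholder cube houses around itself, with the count scaling sublinearly with Population.
; The construction script picks random 2D tile offsets, skips any already in UsedTiles, and scales them to world units for PlaceHouse.
; PlaceHouse line-traces vertically to find the surface, then adds a static mesh component using the world hit location as its relative transform.
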(event EventBeginPlay)

(event Collision|EventActorBeginOverlap
  (params (OtherActor :type Actor%20Object%20Reference)))

(event EventTick
  (params (DeltaSeconds :type Float%20%28single-precision%29)))

(fn ConstructionScript
  (bind _temptile (LocalVariables|GettempTile))
  (bind _temptile_2 (LocalVariables|GettempTile))
  (for _index (range 0 (Math|Float|Truncate (Math|Float|Power (Math|Conversions|ToFloat(Integer) (Variables|Default|Getpopulation)) 0.8)))
    (Class|KismetMathLibrary|Set2D _temptile (Math|Random|RandomFloatinRange -5.0 5.0) (Math|Random|RandomFloatinRange -5.0 5.0))
    (if (not (Utilities|Array|ContainsItem (Variables|Default|GetusedTiles) _temptile))
      (CallFunction|PlaceHouse (* _temptile_2 "(X=256.000000,Y=256.000000)") "/Game/LevelPrototyping/Meshes/SM_ChamferCube.SM_ChamferCube")
      (Utilities|Array|Add (Variables|Default|GetusedTiles) _temptile_2))))

(fn PlaceHouse
  (params (RelativePos :type Vector%202D%20Structure) (Mesh :type Static%20Mesh%20Object%20Reference))
  (bind _returnvalue (Transformation|GetActorLocation))
  (bind _returnvalue_2 (+ _returnvalue RelativePos))
  (bind _outhit (Collision|LineTraceByChannel (+ _returnvalue_2 "0.000000,0.000000,9999999.000000") (+ _returnvalue_2 "0.000000,0.000000,-99999999.000000") "TraceTypeQuery1" false 0 "ForDuration" true "(R=1.000000,G=0.000000,B=0.000000,A=1.000000)" "(R=0.000000,G=1.000000,B=0.000000,A=1.000000)" 2.0))
  (bind _returnvalue_3 (Game|AddComponentbyClass "/Script/Engine.StaticMeshComponent" false (Math|Transform|MakeTransform (.Location (Collision|BreakHitResult _outhit)))))
  (Components|StaticMesh|SetStaticMesh _returnvalue_3 Mesh))