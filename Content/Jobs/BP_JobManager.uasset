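; Job manager actor that generates randomized jobs, each pairing an item with a fuel cost and money reward.
; GenerateRandomJobs appends the requested number of job structs to AvailableJobs, each with a GUID-based ID.
; It draws item data from AvailableItems, rolls cost and reward within Min/Max variables, and fills the {item} placeholder in a random description template.
; The event graph and construction script are empty, so generation relies on external callers.
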(event EventBeginPlay)

(event Collision|EventActorBeginOverlap
  (params (OtherActor :type Actor%20Object%20Reference)))

(event EventTick
  (params (DeltaSeconds :type Float%20%28single-precision%29)))

(fn ConstructionScript)

(fn GenerateRandomJobs
  (params (Amount :type Integer))
  (bind _availableitems (Variables|Default|GetAvailableItems))
  (bind _outitem (Utilities|Array|Random _availableitems))
  (bind (_itemname _itemclass) (Utilities|Struct|BreakSTRUCT_ItemEntry _outitem))
  (for _index (range 1 Amount)
    (Utilities|Array|Add (Variables|Default|GetAvailableJobs) (Utilities|Struct|MakeSTRUCT_JobData (Utilities|String|StringToName (Guid|ToString(Guid) (Guid|NewGuid))) _itemname _itemclass (Math|Random|RandomFloatinRange (Variables|Default|GetMinFuelCost) (Variables|Default|GetMaxFuelCost)) (Math|Random|RandomFloatinRange (Variables|Default|GetMinReward) (Variables|Default|GetMaxReward)) (Utilities|Text|ToText(String) (Utilities|String|Replace (.OutItem (Utilities|Array|Random (Variables|Default|GetJobDescriptionTemplates))) "{item}" (Utilities|String|ToString(Text) _itemname)))))))